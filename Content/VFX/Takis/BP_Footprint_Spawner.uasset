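; Spawner actor that leaves a trail of red footprints under the left foot of its owning BP_ThirdPersonCharacter.
; From BeginPlay, a server-named RPC event calls the spawn event, which line-traces down from the foot socket and places a yaw-aligned BP_FootprintInst_Red at the hit.
; A short function-name timer re-enters that RPC chain to keep the trail going.
; A matching RPC pair destroys every spawner in the world, with debug prints.
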(event Custom|RPC_Server_SpawnFootprints
  (CallFunction|RPCSpawnFootprints))

(event Custom|RPC_SpawnFootprints
  (bind _asbp_third_person_character (Utilities|Casting|CastToBP_ThirdPersonCharacter (Components|GetOwner)))
  (Utilities|IsValid _asbp_third_person_character
    (:Is%20Valid
      (bind (_outhit _returnvalue) (Collision|LineTraceByChannel (.location (Transformation|GetSocketTransform (Variables|/Script/Engine.Character|GetMesh _asbp_third_person_character) "foot_l" "RTS_World")) (+ (.location (Transformation|GetSocketTransform (Variables|/Script/Engine.Character|GetMesh _asbp_third_person_character) "foot_l" "RTS_World")) "0.000000,0.000000,-500.000000") "TraceTypeQuery1" false 0 "None"))
      (if _returnvalue
        (Game|SpawnActorfromClass "/Game/VFX/Takis/BP_FootprintInst_Red.BP_FootprintInst_Red_C" (Math|Transform|MakeTransform (.Location (Collision|BreakHitResult _outhit)) (Math|Rotator|MakeRotator 0.0 0.0 (+ (.yaw (Transformation|GetActorRotation _asbp_third_person_character)) 9e+01)) "1.000000,1.000000,1.000000") "Undefined" "MultiplyWithRoot" 0 0)
        (else
          (Game|SpawnActorfromClass "BP_Footprint_Spawner_C" (Math|Transform|MakeTransform (+ (.location (Transformation|GetSocketTransform (Variables|/Script/Engine.Character|GetMesh _asbp_third_person_character) "foot_l" "RTS_World")) "0.000000,0.000000,-500.000000") (Math|Rotator|MakeRotator 0.0 0.0 (+ (.yaw (Transformation|GetActorRotation _asbp_third_person_character)) 9e+01)) "1.000000,1.000000,1.000000") "Undefined" "MultiplyWithRoot" 0 0)))
      (Utilities|Time|SetTimerbyFunctionName 0 "SpawnFootprintsLoop" 0.2))))

(event Custom|RPC_Server_Destroy
  (CallFunction|RPCDestroy))

(event Custom|RPC_Destroy
  (bind _outactors (Actor|GetAllActorsOfClass "BP_Footprint_Spawner_C"))
  (for _array_element _outactors
    (Development|PrintString "Found spawner!" true true "(R=0.000000,G=0.660000,B=1.000000,A=1.000000)" 4.0)
    (Utilities|IsValid _array_element
      (:Is%20Valid
        (Actor|DestroyActor _array_element)
        (Development|PrintString (Utilities|String|Append (Utilities|String|ToString(Boolean) (Networking|IsServer)) " STEPS ARE GONE") true true "(R=0.728992,G=0.117468,B=1.000000,A=1.000000)" 1e+01)))))

(event EventBeginPlay
  (CallFunction|RPCServerSpawnFootprints))

(fn ConstructionScript)

(fn SpawnFootprintsLoop
  (CallFunction|RPCServerSpawnFootprints))