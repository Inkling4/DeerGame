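; GM_Deer is a game mode that assigns a player ID to each deer player controller passed to it.
; RPC_Server_SetPlayerID casts to Bp_PlayerDeerController, prints the player count for debugging and derives a zero-based ID from that count minus one.
; RPC_SetPlayerID forwards the ID to the controller's own server RPC.
; PostLoginEvent is empty, and nothing in this graph starts the assignment.
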(event Custom|RPC_Server_SetPlayerID
  (params (NewPlayer :type Player%20Controller%20Object%20Reference))
  (bind _returnvalue (Game|GetGameMode))
  (bind _asbp_player_deer_controller (Utilities|Casting|CastToBp_PlayerDeerController NewPlayer))
  (bind _returnvalue_2 (Class|GameModeBase|GetNumPlayers _returnvalue))
  (Development|PrintString (Utilities|String|Append (Utilities|GetDisplayName _returnvalue) " : " (Utilities|String|ToString(Integer) _returnvalue_2)) true true "(R=0.967289,G=1.000000,B=0.273218,A=1.000000)" 15.0)
  (CallFunction|RPCSetPlayerID _asbp_player_deer_controller (- _returnvalue_2 1)))

(event Custom|RPC_SetPlayerID
  (params (NewPlayer :type Bp%20Player%20Deer%20Controller%20Object%20Reference) (PlayerID :type Integer))
  (Default|RPCServerSetPlayerID NewPlayer PlayerID))

(event EventBeginPlay)

(event EventTick
  (params (DeltaSeconds :type Float%20%28single-precision%29)))

(event EventPostLoginEvent
  (params (NewPlayer :type Player%20Controller%20Object%20Reference)))

(fn ConstructionScript)