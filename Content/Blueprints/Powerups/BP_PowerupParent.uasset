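; BP_PowerupParent is a base powerup actor that a third-person character carries as an attached actor and can use.
; UsePowerup routes through a server RPC into RPC_UsePowerup, and destruction follows the same paired-RPC pattern.
; On use, it stores the attach-parent character as TargetActor, clears the UnoReverse flag, detaches its root and hides the mesh.
; It applies no effect of its own and stays alive until the separate destroy event runs.
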(event Custom|RPC_Server_Destroy
  (CallFunction|RPCDestroy))

(event Custom|RPC_Destroy
  (Actor|DestroyActor))

(event Custom|RPC_Server_UsePowerup
  (CallFunction|RPCUsePowerup))

(event Custom|RPC_UsePowerup
  (bind _asbp_third_person_character (Utilities|Casting|CastToBP_ThirdPersonCharacter (Actor|GetAttachParentActor)))
  (Variables|Default|SetTargetActor _asbp_third_person_character)
  (Variables|Default|SetbUnoReverse false)
  (Transformation|DetachFromComponent (Variables|Default|GetDefaultSceneRoot) "KeepRelative" "KeepRelative" "KeepRelative" true)
  (Rendering|SetVisibility (Variables|Default|GetMesh) false true))

(event EventBeginPlay)

(event Collision|EventActorBeginOverlap
  (params (OtherActor :type Actor%20Object%20Reference)))

(event EventTick
  (params (DeltaSeconds :type Float%20%28single-precision%29)))

(fn ConstructionScript)

(fn UsePowerup
  (CallFunction|RPCServerUsePowerup))