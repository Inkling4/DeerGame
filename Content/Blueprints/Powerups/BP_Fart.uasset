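; Fart powerup that propels its target character with repeated impulses for a set duration, with the direction flipped when UnoReverse is set.
; On use it sets an upward velocity and starts a server RPC loop, rescheduled each tick through PowerupLoop until the timer expires and the powerup is destroyed.
; Each pass repeats the impulse through RPC_FartLoop; the force lerp's alpha is always zero, so only FartForceMin applies.
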(event Custom|RPC_Server_FartLoop
  (bind _targetactor (Variables|Default|GetTargetActor))
  (bind _bunoreverse (Variables|Default|GetbUnoReverse))
  (bind _returnvalue (Math|Conversions|ToFloat(Boolean) _bunoreverse))
  (bind _returnvalue_2 (- _returnvalue 0.5))
  (bind _returnvalue_3 (Math|Float|Sign(Float) _returnvalue_2))
  (bind _returnvalue_4 (* _returnvalue_3 -1.0))
  (Utilities|IsValid _targetactor
    (:Is%20Valid
      (Physics|AddImpulse (Variables|/Script/Engine.Character|GetCharacterMovement _targetactor) (Math|Vector|Lerp(Vector) (* (Variables|Default|GetFartForceMin) _returnvalue_4) (* (Variables|Default|GetFartForceMax) _returnvalue_4) (/ 0.0 (Variables|Default|GetFartDuration))) false)
      (CallFunction|RPCFartLoop)
      (bind _returnvalue_5 (Class|KismetSystemLibrary|SetTimerforNextTick 0 "PowerupLoop"))
      (Variables|Default|SetFartTimerHandle _returnvalue_5)
      (Variables|Default|SetFartTimer (- (Variables|Default|GetFartTimer) (Utilities|Time|GetWorldDeltaSeconds))))))

(event Custom|RPC_FartLoop
  (bind _targetactor (Variables|Default|GetTargetActor))
  (bind _bunoreverse (Variables|Default|GetbUnoReverse))
  (bind _returnvalue (Math|Conversions|ToFloat(Boolean) _bunoreverse))
  (bind _returnvalue_2 (- _returnvalue 0.5))
  (bind _returnvalue_3 (Math|Float|Sign(Float) _returnvalue_2))
  (bind _returnvalue_4 (* _returnvalue_3 -1.0))
  (Utilities|IsValid _targetactor
    (:Is%20Valid
      (Physics|AddImpulse (Variables|/Script/Engine.Character|GetCharacterMovement _targetactor) (Math|Vector|Lerp(Vector) (* (Variables|Default|GetFartForceMin) _returnvalue_4) (* (Variables|Default|GetFartForceMax) _returnvalue_4) (/ 0.0 (Variables|Default|GetFartDuration))) false))))

(event EventBeginPlay)

(event Collision|EventActorBeginOverlap
  (params (OtherActor :type Actor%20Object%20Reference)))

(event EventTick
  (params (DeltaSeconds :type Float%20%28single-precision%29)))

(fn ConstructionScript
  (|CallParentFunction))

(fn UsePowerup
  (bind _targetactor (Variables|Default|GetTargetActor))
  (|CallParentFunction)
  (Utilities|IsValid _targetactor
    (:Is%20Valid
      (Variables|Default|SetFartTimer (Variables|Default|GetFartDuration))
      (Variables|/Script/Engine.MovementComponent|SetVelocity (Variables|/Script/Engine.Character|GetCharacterMovement _targetactor) "0.000000,0.000000,100.000000")
      (CallFunction|RPCServerFartLoop))))

(fn PowerupLoop
  (Utilities|IsValid (Variables|Default|GetTargetActor)
    (:Is%20Valid
      (if (> (Variables|Default|GetFartTimer) 0.0)
        (CallFunction|RPCServerFartLoop)
        (else
          (CallFunction|RPCServerDestroy))))))