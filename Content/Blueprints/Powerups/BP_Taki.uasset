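; Takis powerup that speeds up its target actor for a set duration, or slows it down when UnoReverse is set.
; UsePowerup calls the target's server speed RPCs and starts an EndPowerup timer, which later resets speed.
; Use and end pass through server RPCs, with RPC_UseTakis attaching red, or blue if reversed, Niagara footprints to both feet.
; GetTakiSpeed computes scaled speed and acceleration but is not called here.
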(event Custom|RPC_Server_UseTakis
  ;[0.15 0.15 0.15 0.5] Activate Takis Powerup Effect
  (CallFunction|RPCUseTakis)
  (Development|PrintString "server"))

(event Custom|RPC_UseTakis
  (bind _targetactor (Variables|Default|GetTargetActor))
  (bind _mesh (Variables|/Script/Engine.Character|GetMesh _targetactor))
  (bind _returnvalue (Transformation|GetSocketRotation _mesh "foot_l"))
  (bind _returnvalue_2 (Transformation|GetSocketRotation _mesh "foot_l"))
  ;[0.15 0.15 0.15 0.5] Activate Takis Powerup Effect
  (Development|PrintString "client")
  (Utilities|IsValid _targetactor
    (:Is%20Valid
      (if (Variables|Default|GetbUnoReverse)
        (Niagara|SpawnSystemAttached "/Game/VFX/Takis/NS_Footprint_Blue.NS_Footprint_Blue" _mesh "foot_l" "0, 0, 0" (Math|Rotator|MakeRotator 0.0 0.0 (.yaw _returnvalue_2)) "KeepRelativeOffset" true)
        (Niagara|SpawnSystemAttached "/Game/VFX/Takis/NS_Footprint_Blue.NS_Footprint_Blue" _mesh "foot_r" "0, 0, 0" (Math|Rotator|MakeRotator 0.0 0.0 (.yaw _returnvalue_2)) "KeepRelativeOffset" true)
        (else
          (Niagara|SpawnSystemAttached "/Game/VFX/Takis/NS_Footprint_Red.NS_Footprint_Red" _mesh "foot_l" "0, 0, 0" (Math|Rotator|MakeRotator 0.0 0.0 (.yaw _returnvalue)) "KeepRelativeOffset" true)
          (Niagara|SpawnSystemAttached "/Game/VFX/Takis/NS_Footprint_Red.NS_Footprint_Red" _mesh "foot_r" "0, 0, 0" (Math|Rotator|MakeRotator 0.0 0.0 (.yaw _returnvalue)) "KeepRelativeOffset" true)))
      (Development|PrintString "Hello"))))

(event Custom|RPC_Server_EndTakis
  (bind _targetactor (Variables|Default|GetTargetActor))
  (bind _charactermovement (Variables|/Script/Engine.Character|GetCharacterMovement _targetactor))
  ;[0.15 0.15 0.15 0.5] End Takis Powerup Effect
  (Utilities|IsValid _targetactor
    (:Is%20Valid
      (Variables|/Script/Engine.CharacterMovementComponent|SetMaxWalkSpeed _charactermovement (Variables|/Game/ThirdPerson/Blueprints/BP_ThirdPersonCharacter.BP_ThirdPersonCharacter_C|GetDefaultMovementSpeed _targetactor))
      (Variables|/Script/Engine.CharacterMovementComponent|SetMaxAcceleration _charactermovement (Variables|/Game/ThirdPerson/Blueprints/BP_ThirdPersonCharacter.BP_ThirdPersonCharacter_C|GetDefaultAcceleration _targetactor))
      (CallFunction|RPCEndTakis))))

(event Custom|RPC_EndTakis
  (bind _targetactor (Variables|Default|GetTargetActor))
  (bind _charactermovement (Variables|/Script/Engine.Character|GetCharacterMovement _targetactor))
  ;[0.15 0.15 0.15 0.5] End Takis Powerup Effect
  (Utilities|IsValid _targetactor
    (:Is%20Valid
      (Variables|/Script/Engine.CharacterMovementComponent|SetMaxWalkSpeed _charactermovement (Variables|/Game/ThirdPerson/Blueprints/BP_ThirdPersonCharacter.BP_ThirdPersonCharacter_C|GetDefaultMovementSpeed _targetactor))
      (Variables|/Script/Engine.CharacterMovementComponent|SetMaxAcceleration _charactermovement (Variables|/Game/ThirdPerson/Blueprints/BP_ThirdPersonCharacter.BP_ThirdPersonCharacter_C|GetDefaultAcceleration _targetactor)))))

(event EventBeginPlay
  (|CallParentFunction) ; This node is disabled and will not be called.\nDrag off pins to build functionality.
)

(event Collision|EventActorBeginOverlap
  (params (OtherActor :type Actor%20Object%20Reference))
  (|CallParentFunction OtherActor) ; This node is disabled and will not be called.\nDrag off pins to build functionality.
)

(event EventTick
  (params (DeltaSeconds :type Float%20%28single-precision%29))
  (|CallParentFunction DeltaSeconds) ; This node is disabled and will not be called.\nDrag off pins to build functionality.
)

(fn ConstructionScript
  (|CallParentFunction))

(fn UsePowerup
  (bind _targetactor (Variables|Default|GetTargetActor))
  (|CallParentFunction)
  (Utilities|IsValid _targetactor
    (:Is%20Valid
      (Development|PrintString "yippie")
      (if (Variables|Default|GetbUnoReverse)
        (Default|RPCServerDecreaseMovementSpeed _targetactor)
        (Development|PrintString "Decrease")
        (else
          (Default|RPCServerIncreaseMovementSpeed _targetactor)
          (Development|PrintString "Increase")))
      (Utilities|Time|SetTimerbyFunctionName 0 "EndPowerup" (Variables|Default|GetDuration))
      (CallFunction|RPCServerUseTakis))))

(fn EndPowerup
  (bind _targetactor (Variables|Default|GetTargetActor))
  (Utilities|IsValid _targetactor
    (:Is%20Valid
      (Default|RPCServerResetMovementSpeed _targetactor)
      (CallFunction|RPCServerEndTakis))))

(fn GetTakiSpeed
  (bind _targetactor (Variables|Default|GetTargetActor))
  (bind _targetactor_2 (Variables|Default|GetTargetActor))
  (if (Variables|Default|GetbUnoReverse)
    (return (/ (Variables|Default|GetMovementSpeedMult) (Variables|/Game/ThirdPerson/Blueprints/BP_ThirdPersonCharacter.BP_ThirdPersonCharacter_C|GetDefaultMovementSpeed _targetactor_2)) (/ (Variables|Default|GetAccelerationMult) (Variables|/Game/ThirdPerson/Blueprints/BP_ThirdPersonCharacter.BP_ThirdPersonCharacter_C|GetDefaultAcceleration _targetactor_2)))
    (else
      (return (* (Variables|/Game/ThirdPerson/Blueprints/BP_ThirdPersonCharacter.BP_ThirdPersonCharacter_C|GetDefaultMovementSpeed _targetactor) (Variables|Default|GetMovementSpeedMult)) (* (Variables|/Game/ThirdPerson/Blueprints/BP_ThirdPersonCharacter.BP_ThirdPersonCharacter_C|GetDefaultAcceleration _targetactor) (Variables|Default|GetAccelerationMult))))))