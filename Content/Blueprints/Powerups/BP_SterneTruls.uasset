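; Powerup Blueprint "Sterne Truls" that makes its target actor invincible for a set duration.
; UsePowerup runs the parent logic, sets IsInvincible on TargetActor and, only on the server, starts a Duration timer.
; When the timer fires, EndInvincibility calls a server RPC event that relays to RPC_EndInvincibility, which clears the flag if the target is still valid.
; Debug strings print when invincibility starts and ends.
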(event Custom|RPC_Server_EndInvincibility
  (CallFunction|RPCEndInvincibility))

(event Custom|RPC_EndInvincibility
  (bind _targetactor (Variables|Default|GetTargetActor))
  (Utilities|IsValid _targetactor
    (:Is%20Valid
      (Variables|/Game/ThirdPerson/Blueprints/BP_ThirdPersonCharacter.BP_ThirdPersonCharacter_C|SetbIsInvincible _targetactor false)
      (Development|PrintString "No more Sterne Truls :("))))

(event EventBeginPlay
  (|CallParentFunction) ; This node is disabled and will not be called.\nDrag off pins to build functionality.
)

(event Collision|EventActorBeginOverlap
  (params (OtherActor :type Actor%20Object%20Reference))
  (|CallParentFunction OtherActor) ; This node is disabled and will not be called.\nDrag off pins to build functionality.
)

(event EventTick
  (params (DeltaSeconds :type Float%20%28single-precision%29))
  (|CallParentFunction DeltaSeconds) ; This node is disabled and will not be called.\nDrag off pins to build functionality.
)

(fn ConstructionScript
  (|CallParentFunction))

(fn UsePowerup
  (|CallParentFunction)
  (Variables|/Game/ThirdPerson/Blueprints/BP_ThirdPersonCharacter.BP_ThirdPersonCharacter_C|SetbIsInvincible (Variables|Default|GetTargetActor) true)
  (Development|PrintString "Is invincible!")
  (if (Networking|IsServer)
    (Utilities|Time|SetTimerbyFunctionName 0 "EndInvincibility" (Variables|Default|GetDuration))))

(fn EndInvincibility
  (CallFunction|RPCServerEndInvincibility))