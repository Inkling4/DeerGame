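; Powerup spawner that places BP_PowerupBubble actors at random free spawn points.
; BeginPlay calls a server setup event that marks every point available and starts SpawnPowerup.
; SpawnPowerup flags a free point as taken, spawns a bubble with an index and spawner reference, then re-arms a random-delay timer.
; The timer stops when no point is free, and each use of the random pick re-rolls separately.
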(event Custom|RPC_Server_SetupPowerupSpawning
  (Utilities|Array|Clear (Variables|Default|GetbAvailableSpawnPoints))
  (for _index (range 0 (- (Utilities|Array|Length (Variables|PowerupSpawner|GetSpawnPoints)) 1))
    (Utilities|Array|Add (Variables|Default|GetbAvailableSpawnPoints) true))
  (CallFunction|SpawnPowerup))

(event EventBeginPlay
  (CallFunction|RPCServerSetupPowerupSpawning))

(event EventTick
  (params (DeltaSeconds :type Float%20%28single-precision%29)))

(fn ConstructionScript)

(fn SpawnPowerup
  (bind _availablespawnpointindexes (LocalVariables|GetAvailableSpawnPointIndexes))
  (bind _outitem (Utilities|Array|Random _availablespawnpointindexes))
  (Development|PrintString "New Powerup available!")
  (for (_array_element _array_index) (Variables|Default|GetbAvailableSpawnPoints)
    (if _array_element
      (Utilities|Array|Add (LocalVariables|GetAvailableSpawnPointIndexes) _array_index)))
  (if (> (Utilities|Array|Length _availablespawnpointindexes) 0)
    (Utilities|Array|SetArrayElem (Variables|Default|GetbAvailableSpawnPoints) _outitem false)
    (bind _returnvalue (Game|SpawnActorfromClass "/Game/Blueprints/Powerups/BP_PowerupBubble.BP_PowerupBubble_C" (Transformation|GetActorTransform (Utilities|Array|Get(acopy) (Variables|PowerupSpawner|GetSpawnPoints) _outitem)) "Undefined" "MultiplyWithRoot" 0 0))
    (Variables|/Game/Blueprints/Powerups/BP_PowerupBubble.BP_PowerupBubble_C|SetSpawnPointIndex _returnvalue _outitem)
    (Variables|/Game/Blueprints/Powerups/BP_PowerupBubble.BP_PowerupBubble_C|SetPowerupSpawnerRef _returnvalue self)
    (Utilities|Time|SetTimerbyFunctionName 0 "SpawnPowerup" (Math|Random|RandomFloatinRange (Variables|Default|GetSpawnMinTime) (Variables|Default|GetSpawnMaxTime)))))