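; Floating powerup bubble pickup that grants a random powerup to the third-person character that overlaps it.
; Tick bobs the actor with a sine-driven local Z offset.
; Overlap passes through a server RPC to a second RPC, which destroys the bubble, spawns a random class from Powerups attached to the character's left-hand socket and stores it as PowerupRef.
; It then marks its spawn point available again on the spawner, if valid.
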(event OnComponentBeginOverlap(BubbleMesh)
  (params (OverlappedComponent :type Primitive%20Component%20Object%20Reference) (OtherActor :type Actor%20Object%20Reference) (OtherComp :type Primitive%20Component%20Object%20Reference) (OtherBodyIndex :type Integer) (bFromSweep :type Boolean) (SweepResult :type Hit%20Result%20Structure%20%28by%20ref%29))
  (CallFunction|RPCServerGetPowerup OtherActor))

(event Custom|RPC_Server_GetPowerup
  (params (TargetActor :type Actor%20Object%20Reference))
  (CallFunction|RPCGetPowerup TargetActor))

(event Custom|RPC_GetPowerup
  (params (TargetActor :type Actor%20Object%20Reference))
  (bind _powerups (Variables|Powerup|GetPowerups))
  (bind _powerupspawnerref (Variables|Default|GetPowerupSpawnerRef))
  (bind _asbp_third_person_character (Utilities|Casting|CastToBP_ThirdPersonCharacter TargetActor))
  (Variables|Default|SetPlayerRef _asbp_third_person_character)
  (Actor|DestroyActor)
  (bind _returnvalue (Game|SpawnActorfromClass (Utilities|Array|Get(acopy) _powerups (Math|Random|RandomInteger (Utilities|Array|Length _powerups))) (Transformation|GetSocketTransform (Variables|/Script/Engine.Character|GetMesh _asbp_third_person_character) "hand_l" "RTS_World") "Undefined" "MultiplyWithRoot" 0 0))
  (Transformation|AttachComponentToComponent _returnvalue (Variables|/Script/Engine.Character|GetMesh _asbp_third_person_character) "hand_l" "SnapToTarget" "SnapToTarget" "SnapToTarget" true)
  (Variables|/Game/ThirdPerson/Blueprints/BP_ThirdPersonCharacter.BP_ThirdPersonCharacter_C|SetPowerupRef (Variables|Default|GetPlayerRef) _returnvalue)
  (Utilities|IsValid _powerupspawnerref
    (:Is%20Valid
      (Utilities|Array|SetArrayElem (Variables|/Game/Blueprints/Powerups/BP_PowerupSpawner.BP_PowerupSpawner_C|GetbAvailableSpawnPoints _powerupspawnerref) (Variables|Default|GetSpawnPointIndex) true))))

(event EventTick
  (params (DeltaSeconds :type Float%20%28single-precision%29))
  (bind _output_get (Variables|Default|SetDeltaOffset (+ (* DeltaSeconds (Variables|Default|GetBobbingSpeed)) (Variables|Default|GetDeltaOffset))))
  (Transformation|AddActorLocalOffset (Math|Vector|MakeVector 0.0 0.0 (* (Math|Trig|Sin(Radians) _output_get) (Variables|Default|GetBobbingHeight))) false false))

(fn ConstructionScript)