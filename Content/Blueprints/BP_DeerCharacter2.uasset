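; BP_DeerCharacter2 is a deer character Blueprint that takes damage from high-speed crashes.
; Overlapping an actor that implements BPI_Crash fires Crash, which compares horizontal speed to CrashSpeedLimit, ignoring vertical velocity.
; Above the limit, it sends clamped, speed-scaled damage to StatusComp, then DeathCheck tests whether health is depleted.
; Death and crash outcomes are only reported through debug prints.
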(event EventBeginPlay)

(event Collision|EventActorBeginOverlap
  (params (OtherActor :type Actor%20Object%20Reference))
  ;[0.15 0.15 0.15 0.5] Activates event "crash" if the character collides with an actor with the BPI_Crash interface.
  (if (Utilities|DoesObjectImplementInterface OtherActor "/Game/Blueprints/Interfaces/BPI_Crash.BPI_Crash_C")
    (CallFunction|Crash)))

(event EventDeathCheck
  ;[0.15 0.15 0.15 0.5] Death Check function
  (bind _isdead (CallFunction|IsCharacterDead))
  (if _isdead
    (Development|PrintString "You are dead! Not big surprise.")))

(event EventCrash
  (bind _returnvalue (Transformation|GetVelocity))
  (bind _crashspeedlimit (Variables|Default|GetCrashSpeedLimit))
  (bind (_x _y) (Math|Vector|BreakVector _returnvalue))
  (bind _returnvalue_2 (Class|KismetMathLibrary|Hypotenuse _x _y))
  ;[0.15 0.15 0.15 0.5] Checks if speed is high enough to take damage. Does not check vertical speed.
  (if (>= _returnvalue_2 _crashspeedlimit)
    (Development|PrintString "You would take damage from this crash!")
    (Class|StatusComponent|TakeDamage (Variables|Default|GetStatusComp) (Math|Float|Truncate (Math|Float|Clamp(Float) (+ (/ (- _returnvalue_2 _crashspeedlimit) 7e+01) 5.0) 5.0 5e+01)))
    (Default|DeathCheck self)
    (else
      (Development|PrintString "You would not take damage from this crash."))))

(fn ConstructionScript)

(fn IsCharacterDead
  (if (<= (Class|StatusComponent|GetHealth (Variables|Default|GetStatusComp)) 0)
    (return true)
    (else
      (return false))))