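; Player deer character Blueprint that manages health, crash damage and death.
; On begin play it creates a health bar widget, refreshed every tick from the StatusComponent's health.
; Overlapping a BPI_Crash actor triggers a crash check, where horizontal speed above CrashSpeedLimit deals clamped, speed-scaled damage through StatusComponent.
; At zero health it disables input and, after a short delay, opens the Game Over level.
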(event EventBeginPlay
  ;[0.15 0.15 0.15 0.5] Creates Health Bar
  (bind _returnvalue (UserInterface|CreateWidget "/Game/Blueprints/UI_PlayerHealthBar.UI_PlayerHealthBar_C" (Game|GetPlayerController 0)))
  (bind _output_get (Variables|Default|SetHealthBarWidget _returnvalue))
  (UserInterface|Viewport|AddtoViewport _output_get 0)
  (Default|UpdateHealthBar _returnvalue 1e+02))

(event Collision|EventActorBeginOverlap
  (params (OtherActor :type Actor%20Object%20Reference))
  ;[0.15 0.15 0.15 0.5] Activates event "crash" if the character collides with an actor with the BPI_Crash interface.
  (if (Utilities|DoesObjectImplementInterface OtherActor "/Game/Blueprints/Interfaces/BPI_Crash.BPI_Crash_C")
    (CallFunction|Crash)))

(event EventDeathCheck
  ;[0.15 0.15 0.15 0.5] Death Check function
  (bind _isdead (CallFunction|IsCharacterDead))
  (if _isdead
    (Input|DisableInput (Game|GetPlayerController 0))
    (Utilities|FlowControl|Delay 0.7)
    (Game|OpenLevel(byObjectReference) "/Game/Levels/LVL_GameOver.LVL_GameOver")))

(event EventTick
  (params (DeltaSeconds :type Float%20%28single-precision%29))
  ;[0.15 0.15 0.15 0.5] Updates the health bar every tick
  (Default|UpdateHealthBar (Variables|Default|GetHealthBarWidget) (Math|Conversions|ToFloat(Integer) (Class|StatusComponent|GetHealth (Variables|Default|GetStatusComponent)))))

(event EventCrash
  (bind _returnvalue (Transformation|GetVelocity))
  (bind _crashspeedlimit (Variables|Default|GetCrashSpeedLimit))
  (bind (_x _y) (Math|Vector|BreakVector _returnvalue))
  (bind _returnvalue_2 (Class|KismetMathLibrary|Hypotenuse _x _y))
  ;[0.15 0.15 0.15 0.5] Checks if speed is high enough to take damage. Does not check vertical speed.
  (if (>= _returnvalue_2 _crashspeedlimit)
    (Development|PrintString "You would take damage from this crash!")
    (Class|StatusComponent|TakeDamage (Variables|Default|GetStatusComponent) (Math|Float|Truncate (Math|Float|Clamp(Float) (+ (/ (- _returnvalue_2 _crashspeedlimit) 7e+01) 5.0) 5.0 5e+01)))
    (CallFunction|DeathCheck)
    (else
      (Development|PrintString "You would not take damage from this crash."))))

(fn ConstructionScript)

(fn IsCharacterDead
  (if (<= (Class|StatusComponent|GetHealth (Variables|Default|GetStatusComponent)) 0)
    (return true)
    (else
      (return false))))